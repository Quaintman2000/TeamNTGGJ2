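; AI controller for the monster that hunts the player by sound and runs BT_Monster on possess.
; A looping timer compares the pawn's distance to the player's current noise radius, setting HeardSound and PlayerActor on the Blackboard when within range.
; Once out of range, a one-shot investigation timer starts, then clears both keys on expiry to end the pursuit.
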(event Custom|StartEnemyTimer
  (bind _blackboard (Variables|Default|GetBlackboard))
  (AI|Components|Blackboard|SetValueasBool _blackboard (Variables|Default|GetHeard%20Sound) false)
  (AI|Components|Blackboard|SetValueasObject _blackboard (Variables|Default|GetPlayer%20Actor) 0)
  (Variables|Default|SetInvestigating false)
  (Development|PrintString "Dont hear player"))

(event Custom|Check%20for%20Player
  (bind _blackboard (Variables|Default|GetBlackboard))
  (bind _playercharacter (Variables|Default|GetPlayerCharacter))
  (bind _range (Default|GetCurrentNoiseRadius _playercharacter))
  (if (<= (Math|Vector|Distance(Vector) (Transformation|GetActorLocation (Pawn|GetControlledPawn self)) (Transformation|GetActorLocation _playercharacter)) _range) ; If the monster is within the noise radius
    (Utilities|Time|ClearandInvalidateTimerbyHandle (Variables|Default|GetEnemy%20Timer)) ; Stop the investigation timer and start chase
    (AI|Components|Blackboard|SetValueasBool _blackboard (Variables|Default|GetHeard%20Sound) true)
    (AI|Components|Blackboard|SetValueasObject _blackboard (Variables|Default|GetPlayer%20Actor) (Variables|Default|GetPlayerCharacter))
    (Development|PrintString "I hear the player")
    (elif (ScalableFloat|GetValueasBool (Variables|Default|GetBlackboard) (Variables|Default|GetHeard%20Sound)) ; If we don't hear the player now but we did recently
      (if (not (Variables|Default|GetInvestigating))
        (bind _returnvalue (Utilities|Time|SetTimerbyEvent (delegate Custom|StartEnemyTimer) (Variables|Default|GetInvestigate%20Timer)))
        (bind _output_get (Variables|Default|SetEnemy%20Timer _returnvalue))
        (Variables|Default|SetInvestigating true)
        (Development|PrintString "Where is the player?")
        (Development|PrintString (Utilities|String|ToString(Float) (Utilities|Time|GetTimerRemainingTimebyHandle _output_get))))
      (else
        (Development|PrintString "Dont hear player")))))

(event EventBeginPlay
  (bind _returnvalue (Actor|GetActorOfClass "/Game/FirstPerson/Blueprints/BP_FirstPersonCharacter.BP_FirstPersonCharacter_C"))
  (Variables|Default|SetPlayerCharacter _returnvalue)
  (Utilities|Time|SetTimerbyEvent (delegate Custom|Check%20for%20Player) 1.0 true))

(event EventPossess
  (params (PossessedPawn :type Pawn%20Object%20Reference))
  (AI|RunBehaviorTree "/Game/Blueprints/Monster/BT_Monster.BT_Monster"))

(fn ConstructionScript)