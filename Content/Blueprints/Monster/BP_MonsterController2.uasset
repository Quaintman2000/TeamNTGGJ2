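; AI controller for the monster that runs BT_Monster on possession and gives it a simple sense of hearing.
; A looping timer compares the monster's distance to the player against the player's current noise radius, writing heard-sound and player-actor Blackboard keys when within range.
; Losing the sound starts a one-shot investigation timer that clears both keys on expiry; hearing the player again does not cancel it.
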(event Custom|HearCheckForPlayer
  (bind _range (Default|GetCurrentNoiseRadius (Variables|Default|GetPlayerCharacter)))
  (if (<= (Math|Vector|Distance(Vector) (Transformation|GetActorLocation (Pawn|GetControlledPawn self)) (Transformation|GetActorLocation (Variables|Default|GetPlayerCharacter))) _range)
    (AI|Components|Blackboard|SetValueasBool (Variables|Default|GetBlackboard) (Variables|Default|GetHeard%20Sound%20Key) true)
    (AI|Components|Blackboard|SetValueasObject (Variables|Default|GetBlackboard) (Variables|Default|GetPlayerActorKey) (Variables|Default|GetPlayerCharacter))
    (Development|PrintString "I hear the player")
    (elif (ScalableFloat|GetValueasBool (Variables|Default|GetBlackboard) (Variables|Default|GetHeard%20Sound%20Key))
      (if (not (Variables|Default|GetIsInvestigating))
        (bind _returnvalue (Utilities|Time|SetTimerbyEvent (delegate Custom|OnInvestigationEnd) (Variables|Default|GetInvestigationTime)))
        (Variables|Default|SetInvestigationTimer _returnvalue)
        (Variables|Default|SetIsInvestigating true)
        (Development|PrintString "Where is the player?")))))

(event Custom|OnInvestigationEnd
  (AI|Components|Blackboard|SetValueasBool (Variables|Default|GetBlackboard) (Variables|Default|GetHeard%20Sound%20Key) false)
  (AI|Components|Blackboard|SetValueasObject (Variables|Default|GetBlackboard) (Variables|Default|GetPlayerActorKey) 0)
  (Variables|Default|SetIsInvestigating false)
  (Development|PrintString "Dont hear player"))

(event EventBeginPlay
  (bind _returnvalue (Actor|GetActorOfClass "/Game/FirstPerson/Blueprints/BP_FirstPersonCharacter.BP_FirstPersonCharacter_C"))
  (Variables|Default|SetPlayerCharacter _returnvalue)
  (Utilities|Time|SetTimerbyEvent (delegate Custom|HearCheckForPlayer) (Variables|Default|GetHear%20Check%20Interval) true))

(event EventPossess
  (params (PossessedPawn :type Pawn%20Object%20Reference))
  (AI|RunBehaviorTree "/Game/Blueprints/Monster/BT_Monster.BT_Monster"))

(fn ConstructionScript)